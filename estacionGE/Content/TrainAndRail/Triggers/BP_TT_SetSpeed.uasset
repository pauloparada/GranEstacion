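; Train-and-rail trigger that changes a carriage's speed when triggered.
; Its internal trigger event optionally overrides the carriage's max speed, current speed, or both, each gated by its own flag.
; The construction script optionally adds a centered text label previewing the enabled values in the editor, hidden in game.
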(event EventBeginPlay)

(event Collision|EventActorBeginOverlap
  (params (OtherActor :type Actor%20Object%20Reference)))

(event EventInternalTriggerEvent
  (params (Bogie :type AC%20Bogie%20Object%20Reference) (Carriage :type BP%20Train%20Carriage%20Object%20Reference))
  (Utilities|FlowControl|Sequence
    (:then_0
      (if (Variables|SpeedTriggerSettings|GetSetMaxSpeed)
        (Variables|/Game/TrainAndRail/Blueprints/BP_TrainCarriage.BP_TrainCarriage_C|SetMaxSpeed Carriage (Variables|SpeedTriggerSettings|GetMaxSpeed))))
    (:then_1
      (if (Variables|SpeedTriggerSettings|GetSetCurrentSpeed)
        (Variables|/Game/TrainAndRail/Blueprints/BP_TrainCarriage.BP_TrainCarriage_C|SetCurrentSpeed Carriage (Variables|SpeedTriggerSettings|GetCurrentSpeed))))))

(event EventTick
  (params (DeltaSeconds :type Float%20%28single-precision%29))
  (|CallParentFunction 0.0))

(fn ConstructionScript
  (|CallParentFunction)
  (CallFunction|SetupInfoText))

(fn SetupInfoText
  (if (Variables|SpeedTriggerInfoSettings|GetDisplayInfoText)
    (bind _returnvalue (AddComponent|AddTextRenderComponent false (Math|Transform|MakeTransform (Math|Vector|MakeVector 0.0 0.0 (Variables|SpeedTriggerInfoSettings|GetInfoTextOffsetZ)))))
    (Rendering|Components|TextRender|SetText _returnvalue (Utilities|Text|FormatText "{a}{b}" (select (Variables|SpeedTriggerSettings|GetSetMaxSpeed) (Utilities|Text|FormatText "Max: {ms}<br>" (Variables|SpeedTriggerSettings|GetMaxSpeed)) "") (select (Variables|SpeedTriggerSettings|GetSetCurrentSpeed) (Utilities|Text|FormatText "Current: {cs}" (Variables|SpeedTriggerSettings|GetCurrentSpeed)) "")))
    (Rendering|Components|TextRender|SetWorldSize _returnvalue (Variables|SpeedTriggerInfoSettings|GetInfoTextFontSize))
    (Rendering|Components|TextRender|SetHorizontalAlignment _returnvalue "EHTA_Center")
    (Rendering|Components|TextRender|SetTextRenderColor _returnvalue (Variables|SpeedTriggerInfoSettings|GetInfoDisplayColor))
    (Development|SetHiddeninGame _returnvalue true true)))