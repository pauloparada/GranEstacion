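; Train track Blueprint that fits its spline to the terrain at construction time.
; An elevated marker spline supplies points and optional tangents, which are copied into the inherited default track spline.
; Each point is line-traced down onto the surface, or simply lowered by the marker height, with optional highlight spheres, before the parent construction script runs.
; Functions for generating evenly spaced or subdivided points exist but are not called here.
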(event EventBeginPlay)

(event Collision|EventActorBeginOverlap
  (params (OtherActor :type Actor%20Object%20Reference)))

(event EventTick
  (params (DeltaSeconds :type Float%20%28single-precision%29)))

(fn ConstructionScript
  (CallFunction|InitalizeTerrainTrack)
  (Transformation|SetRelativeLocation (Variables|Default|GetTerrainSplineMarker) (Math|Vector|MakeVector 0.0 0.0 (Variables|TerrainTrackSettings|GetMarkerSplineHeight)) false true)
  (CallFunction|CopySplinePoints)
  (CallFunction|TracePoints)
  (if (Variables|TerrainTrackSettings|GetHighlightSplinePoints)
    (CallFunction|AddPointSpheres))
  (|CallParentFunction))

(fn InitalizeTerrainTrack
  (bind _output_get (Variables|TerrainTrackSettings|SetTerrainSpline (Variables|Default|GetDefaultTrackSpline)))
  (Spline|ClearSplinePoints _output_get false))

(fn AddSplinePoints
  (Utilities|FlowControl|Sequence
    (:then_0
      ;[1 1 1] Wipe all the current points
      (Spline|ClearSplinePoints (Variables|TerrainTrackSettings|GetTerrainSpline) false))
    (:then_1
      ;[1 1 1] Setup spacing and the spline length
      (if (< (Variables|TerrainTrackSettings|GetPointCount) 3)
        (Variables|TerrainTrackSettings|SetPointCount 3)
        (Development|PrintString "Point count less than 3, reset to 3"))
      (LocalVariables|SetSplineLength (CallFunction|GetDistanceBetweenLocations (Variables|TerrainTrackSettings|GetStartPoint) (Variables|TerrainTrackSettings|GetEndPoint)))
      (LocalVariables|SetPointDistance (/ (LocalVariables|GetSplineLength) (Math|Conversions|ToFloat(Integer) (- (Variables|TerrainTrackSettings|GetPointCount) 1)))))
    (:then_2
      (for _index (range 0 (- (Variables|TerrainTrackSettings|GetPointCount) 1))
        (LocalVariables|SetCurrentSplinePoint _index)
        (Utilities|FlowControl|Sequence
          (:then_0
            (LocalVariables|SetPosSet false))
          (:then_1
            ;[1 1 1] If this is the start, we want to use the points from the gizmo, transform the gizmo from local position into world position
            (if (and (== (LocalVariables|GetCurrentSplinePoint) 0) (Variables|TerrainTrackSettings|GetUseTraceOnStartPoint))
              (LocalVariables|SetPointLocation (Math|Transform|TransformLocation (Transformation|GetWorldTransform (Variables|Default|GetScene self)) (Variables|TerrainTrackSettings|GetStartPoint)))
              (LocalVariables|SetPosSet true)))
          (:then_2
            ;[1 1 1] Use the end point gizmo
            (if (and (== (LocalVariables|GetCurrentSplinePoint) (- (Variables|TerrainTrackSettings|GetPointCount) 1)) (Variables|TerrainTrackSettings|GetUseTraceOnEndPoint))
              (LocalVariables|SetPointLocation (Math|Transform|TransformLocation (Transformation|GetWorldTransform (Variables|Default|GetScene self)) (Variables|TerrainTrackSettings|GetEndPoint)))
              (LocalVariables|SetPosSet true)))
          (:then_3
            ;[1 1 1] If this is any other point, generate its position on the spline
            (if (not (LocalVariables|GetPosSet))
              (LocalVariables|SetPointLocation (+ (Variables|TerrainTrackSettings|GetStartPoint) (* (Math|Vector|GetForwardVector (Variables|Default|GetScene self)) (* (LocalVariables|GetCurrentSplinePoint) (LocalVariables|GetPointDistance)))))
              ;[1 1 1] Line trace from above the generated position, if we hit something use that as the new position for this point
              (bind (_outhit _returnvalue) (Collision|LineTraceByChannel (+ (LocalVariables|GetPointLocation) (Math|Vector|MakeVector 0.0 0.0 (Variables|TerrainTrackSettings|GetTraceOffsetAbove)) (Transformation|GetWorldLocation (Variables|Default|GetScene self))) (- (+ (LocalVariables|GetPointLocation) (Math|Vector|MakeVector 0.0 0.0 (Variables|TerrainTrackSettings|GetTraceOffsetAbove)) (Transformation|GetWorldLocation (Variables|Default|GetScene self))) (Math|Vector|MakeVector 0.0 0.0 (Variables|TerrainTrackSettings|GetTraceDistance))) "TraceTypeQuery1" false 0 "None"))
              (if _returnvalue
                (LocalVariables|SetPointLocation (.Location (Collision|BreakHitResult _outhit))))))
          (:then_4
            ;[1 1 1] Set the position for the new spline point
            (Spline|AddSplinePoint (Variables|TerrainTrackSettings|GetTerrainSpline) (+ (LocalVariables|GetPointLocation) (Math|Vector|SelectVector "0, 0,100.000000" "0, 0, 0" (== (LocalVariables|GetCurrentSplinePoint) 1))) "World" false)))))
    (:then_3
      (Spline|UpdateSpline (Variables|TerrainTrackSettings|GetTerrainSpline)))))

(fn CreateNewSplinePoints
  (bind _terrainsplinemarker (Variables|Default|GetTerrainSplineMarker))
  (bind _pointcountpersection (Variables|TerrainTrackSettings|GetPointCountPerSection))
  (bind _terrainsplinemarker_2 (Variables|Default|GetTerrainSplineMarker))
  (bind (_startindex _endindex) (Utilities|GetSplinePointLoopVars _terrainsplinemarker))
  (LocalVariables|SetPointSampleCount (Math|Integer|SelectInt _pointcountpersection 0 (>= _pointcountpersection 0)))
  (for _index (range _startindex (- _endindex 1))
    (bind _output_get (LocalVariables|SetCurrentPointIndex _index))
    (LocalVariables|SetNextPointIndex (+ _output_get 1))
    (Utilities|FlowControl|Sequence
      (:then_0
        (LocalVariables|SetCurrentPointDistance (Spline|GetDistanceAlongSplineatSplinePoint _terrainsplinemarker_2 (LocalVariables|GetCurrentPointIndex)))
        (LocalVariables|SetNextPointDistance (Spline|GetDistanceAlongSplineatSplinePoint _terrainsplinemarker_2 (LocalVariables|GetNextPointIndex))))
      (:then_1
        (LocalVariables|SetDistanceIncrease (/ (- (LocalVariables|GetNextPointDistance) (LocalVariables|GetCurrentPointDistance)) (Math|Conversions|ToFloat(Integer) (+ (LocalVariables|GetPointSampleCount) 1))))
        (Development|PrintString (Utilities|String|ToString(Text) (Utilities|Text|FormatText "Current point {cp} at distance {cpd} , next point {npi} at dist {npd} so inc is {inc}" (LocalVariables|GetCurrentPointIndex) (LocalVariables|GetCurrentPointDistance) (LocalVariables|GetNextPointIndex) (LocalVariables|GetNextPointDistance) (LocalVariables|GetDistanceIncrease)))))
      (:then_2
        (for _index_2 (range 1 (LocalVariables|GetPointSampleCount))
          (Development|PrintString (Utilities|String|ToString(Text) (Utilities|Text|FormatText "Adding new point {npi} at distance {npd}" _index_2 (+ (* _index_2 (LocalVariables|GetDistanceIncrease)) (LocalVariables|GetCurrentPointDistance)))))
          (Spline|AddSplinePoint (Variables|TerrainTrackSettings|GetTerrainSpline) (Spline|GetLocationatDistanceAlongSpline (Variables|Default|GetTerrainSplineMarker) (+ (* _index_2 (LocalVariables|GetDistanceIncrease)) (LocalVariables|GetCurrentPointDistance)) "World") "World" false)))))
  (Spline|UpdateSpline (Variables|TerrainTrackSettings|GetTerrainSpline)))

(fn CopySplinePoints
  (bind _terrainsplinemarker (Variables|Default|GetTerrainSplineMarker))
  (bind _terrainspline (Variables|TerrainTrackSettings|GetTerrainSpline))
  (bind _terrainsplinemarker_2 (Variables|Default|GetTerrainSplineMarker))
  (bind (_startindex _endindex) (Utilities|GetSplinePointLoopVars _terrainsplinemarker))
  (Spline|ClearSplinePoints (Variables|TerrainTrackSettings|GetTerrainSpline) false)
  (for _index (range _startindex _endindex)
    (Spline|AddSplinePoint _terrainspline (Spline|GetLocationatSplinePoint _terrainsplinemarker_2 _index "World") "World" false)
    (if (Variables|TerrainTrackSettings|GetCopyTangents)
      (Spline|SetTangentatSplinePoint _terrainspline _index (Spline|GetTangentatSplinePoint _terrainsplinemarker_2 _index "World") "World" false :!label _label)
      (elif (and (Variables|TerrainTrackSettings|GetCopyStartPointTangent) (== _index 0))
        (goto _label)
        (elif (and (Variables|TerrainTrackSettings|GetCopyEndPointTangent) (== _index _endindex))
          (goto _label)))))
  (Spline|UpdateSpline _terrainspline))

(fn TracePoints
  (bind _terrainspline (Variables|TerrainTrackSettings|GetTerrainSpline))
  (bind (_startindex _endindex) (Utilities|GetSplinePointLoopVars _terrainspline))
  (for _index (range _startindex _endindex)
    (if (Variables|TerrainTrackSettings|GetDoNotTrace)
      (Spline|SetLocationatSplinePoint _terrainspline _index (- (Spline|GetLocationatSplinePoint _terrainspline _index "World") (Math|Vector|MakeVector 0.0 0.0 (Variables|TerrainTrackSettings|GetMarkerSplineHeight))) "World" false)
      (else
        (bind (_outhit _returnvalue) (Collision|LineTraceByChannel (+ (Spline|GetLocationatSplinePoint _terrainspline _index "World") (Math|Vector|MakeVector 0.0 0.0 (Variables|TerrainTrackSettings|GetTraceOffsetAbove))) (- (+ (Spline|GetLocationatSplinePoint _terrainspline _index "World") (Math|Vector|MakeVector 0.0 0.0 (Variables|TerrainTrackSettings|GetTraceOffsetAbove))) (Math|Vector|MakeVector 0.0 0.0 (Variables|TerrainTrackSettings|GetTraceDistance))) "TraceTypeQuery1" true 0 "ForDuration" true "(R=1.000000,G=0.000000,B=0.000000,A=1.000000)" "(R=0.000000,G=1.000000,B=0.000000,A=1.000000)" 2.0))
        (if _returnvalue
          (Spline|SetLocationatSplinePoint _terrainspline _index (.Location (Collision|BreakHitResult _outhit)) "World" false)))))
  (Spline|UpdateSpline _terrainspline))

(fn AddPointSpheres
  (bind _defaulttrackspline (Variables|Default|GetDefaultTrackSpline))
  (bind (_startindex _endindex) (Utilities|GetSplinePointLoopVars _defaulttrackspline))
  (for _index (range _startindex _endindex)
    (bind _returnvalue (AddComponent|AddSphereComponent false (Math|Transform|MakeTransform (Spline|GetLocationatSplinePoint _defaulttrackspline _index "Local"))))
    (Components|Sphere|SetSphereRadius _returnvalue (Variables|TerrainTrackSettings|GetHighlightSplinePointSize) false)
    (Collision|SetCollisionEnabled _returnvalue "NoCollision")))