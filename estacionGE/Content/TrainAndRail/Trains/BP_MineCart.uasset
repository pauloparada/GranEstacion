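; Mine cart train vehicle that feeds wheel speed to its own animation blueprint and can perform a scripted jump.
; SetJumpSettings defines duration and an offset transform, and StartJump caches the original scale.
; While jumping, Tick blends the current location and rotation, plus the cached scale, toward that additive offset, with alpha rising to the halfway peak and falling back until the jump ends.
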(event EventBeginPlay
  (|CallParentFunction))

(event Collision|EventActorBeginOverlap
  (params (OtherActor :type Actor%20Object%20Reference)))

(event EventTick
  (params (DeltaSeconds :type Float%20%28single-precision%29))
  (|CallParentFunction DeltaSeconds)
  ;[1 1 1] Tick the jump if we are jumping
  (if (Variables|JumpSettings|GetIsJumping)
    (CallFunction|TickJump DeltaSeconds)))

(event EventUpdateAnimations
  ;[1 1 1] Overwrite the update animation function for the mine cart since we are using a different anim blueprint
  (bind _asanimbp_mine_cart (Utilities|Casting|CastToANIMBP_MineCart (Components|SkeletalMesh|GetAnimInstance (Variables|Default|GetFrontBogieMesh))))
  (Variables|/Game/TrainAndRail/Models/MineCart/ANIMBP_MineCart.ANIMBP_MineCart_C|SetWheelSpeed _asanimbp_mine_cart (CallFunction|GetWheelSpeed)))

(fn ConstructionScript
  (|CallParentFunction))

(fn StartJump
  (Variables|JumpSettings|SetIsJumping true)
  (Variables|JumpSettings|SetJumpCurrentTime 0.0)
  ;[1 1 1] Store the scale so we can restore later
  (Variables|JumpSettings|SetOriginalScale (Transformation|GetActorScale3D self)))

(fn TickJump
  (params (DeltaSeconds :type Float%20%28single-precision%29%20%28by%20ref%29))
  (bind _returnvalue (Transformation|GetActorTransform))
  (bind _jumptransform (Variables|JumpSettings|GetJumpTransform))
  (bind (_location _rotation) (Math|Transform|BreakTransform _returnvalue))
  (bind (_location_2 _rotation_2 _scale) (Math|Transform|BreakTransform _jumptransform))
  ;[1 1 1] Fade into transform or fade back to normal?
  (bind _output_get (LocalVariables|SetFadeIn (< (Variables|JumpSettings|GetJumpCurrentTime) (Variables|JumpSettings|GetJumpPeak))))
  (if _output_get
    ;[1 1 1] Fade in goes from 0 to 1. Fade out from 1 to 0
    (LocalVariables|SetAlpha (/ (Variables|JumpSettings|GetJumpCurrentTime) (Variables|JumpSettings|GetJumpPeak)))
    (else
      (LocalVariables|SetAlpha (- 1.0 (/ (- (Variables|JumpSettings|GetJumpCurrentTime) (Variables|JumpSettings|GetJumpPeak)) (Variables|JumpSettings|GetJumpPeak))))))
  ;[1 1 1] Set the original scale so we have the correct base transform
  (LocalVariables|SetSourceTransform (Math|Transform|MakeTransform _location _rotation (Variables|JumpSettings|GetOriginalScale)))
  ;[1 1 1] Grab the current transform, then build the final transform
  (LocalVariables|SetTargetTransform (Math|Transform|MakeTransform (+ (.Location (Math|Transform|BreakTransform (LocalVariables|GetSourceTransform))) _location_2) (Math|Rotator|CombineRotators (.Rotation (Math|Transform|BreakTransform (LocalVariables|GetSourceTransform))) _rotation_2) (+ (.Scale (Math|Transform|BreakTransform (LocalVariables|GetSourceTransform))) _scale)))
  ;[1 1 1] Lerp between current transform and the target transform
  (Transformation|SetActorTransform (Math|Transform|Lerp(Transform) (LocalVariables|GetSourceTransform) (LocalVariables|GetTargetTransform) (LocalVariables|GetAlpha)))
  ;[1 1 1] Update the jump run time and end if enough time has passed
  (bind _output_get_2 (Variables|JumpSettings|SetJumpCurrentTime (+ DeltaSeconds (Variables|JumpSettings|GetJumpCurrentTime))))
  (if (>= _output_get_2 (Variables|JumpSettings|GetJumpRunTime))
    (CallFunction|EndJump)))

(fn EndJump
  (Variables|JumpSettings|SetIsJumping false))

(fn SetJumpSettings
  (params (JumpDuration :type Float%20%28single-precision%29) (JumpTransform :type Transform))
  (Variables|JumpSettings|SetJumpRunTime JumpDuration)
  (Variables|JumpSettings|SetJumpTransform JumpTransform)
  (Variables|JumpSettings|SetJumpPeak (/ (Variables|JumpSettings|GetJumpRunTime) 2.0)))